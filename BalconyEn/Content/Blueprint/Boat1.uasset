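; Boat actor that bobs and rocks its static mesh in an idle floating motion.
; BeginPlay seeds a random timer offset so each instance starts at a different phase.
; Tick advances the timer and uses its sine to add a small local pitch and a vertical world offset.
; Both offsets accumulate per frame without delta-time scaling, so the motion's amplitude depends on frame rate.
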(event EventBeginPlay
  (Variables|Default|SetTimer (* (Math|Random|RandomFloat) 1e+01)))

(event Collision|EventActorBeginOverlap
  (params (OtherActor :type Actor%20Object%20Reference)))

(event EventTick
  (params (DeltaSeconds :type Float%20%28single-precision%29))
  (bind _staticmesh (Variables|Default|GetStaticMesh))
  (bind _returnvalue (Transformation|GetWorldLocation _staticmesh))
  (bind (_x _y _z) (Math|Vector|BreakVector _returnvalue))
  (bind _output_get (Variables|Default|SetTimer (+ (* DeltaSeconds 2.0) (Variables|Default|GetTimer))))
  (Transformation|AddLocalRotation _staticmesh (Math|Rotator|MakeRotator 0.0 (* (Math|Trig|Sin(Radians) _output_get) 0.05) 0.0) false false)
  (Transformation|SetWorldLocation _staticmesh (Math|Vector|MakeVector _x _y (+ _z (Math|Trig|Sin(Radians) _output_get))) false false))

(fn ConstructionScript)